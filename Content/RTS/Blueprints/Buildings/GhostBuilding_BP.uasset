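; Ghost building actor for an RTS build mode, previewing a chosen building at the cursor's grid-snapped world position.
; ConstructBuilding briefly spawns the building class to read its display mesh and construction proxy, resets the ghost, then destroys that instance.
; OnSpawn applies the mesh with a ghost material and flags build mode on the GodsEye pawn.
; A gated Tick moves the ghost until KillGhost closes it and clears state.
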(event `OnSpawn`
  (params (DisplayMesh :type "StaticMesh Object Reference") (`Building Type` :type "/Game/RTS/Blueprints/Buildings/BuildingMaster_BP Class Reference") (`Construction Proxy` :type "/Game/RTS/Blueprints/Construction/ConstructionProxy_BP Class Reference"))
  (if (not (`self.IsActive`))
    (bind _output_get (set `self.DisplayMesh` DisplayMesh))
    (set `self.ConstructionProxy` `Construction Proxy`)
    (set `self.BuildingType` `Building Type`)
    (set `self.IsActive` true)
    (set `/Game/RTS/Blueprints/GodsEye_Pawn.BuildModeActive` true (`self.GodsEyePawnReference`))
    (`StaticMeshComponent.SetStaticMesh` (`self.GhostBuilding_Mesh`) _output_get)
    (for (_ _array_index) (`MeshComponent.GetMaterials` (`self.GhostBuilding_Mesh`))
      (`PrimitiveComponent.SetMaterial` (`self.GhostBuilding_Mesh`) _array_index "/Game/RTS/Blueprints/Ghost_Material.Ghost_Material"))))

(event `KillGhost`
  ;[1 1 1] Kill
  (set `self.DisplayMesh` null)
  (`self.CloseTickGate`)
  (set `self.ConstructionProxy` null)
  (set `self.BuildingType` null)
  (set `self.IsActive` false)
  (set `/Game/RTS/Blueprints/GodsEye_Pawn.BuildModeActive` false (`self.GodsEyePawnReference`)))

(event `/Game/RTS/UI/HUD_Interface.Construct Building`
  (params (`Main Building` :type "/Game/RTS/Blueprints/Buildings/BuildingMaster_BP Class Reference"))
  (bind _returnvalue (`|SpawnActorFromClass` `Main Building` (`KismetMathLibrary.MakeTransform` (0.0 0.0 0.0)) "Undefined" "OverrideRootScale" null (`self.ControllerReference`) null))
  (`|ExecutionSequence`
    (:`then_0`
      (bind _asbuilding_master_bp (castclass `/Game/RTS/Blueprints/Buildings/BuildingMaster_BP` `Main Building`))
      (`self.KillGhost`)
      (`self.OnSpawn` (`/Game/RTS/Blueprints/Buildings/BuildingMaster_BP.DisplayMesh` _returnvalue) _asbuilding_master_bp (`/Game/RTS/Blueprints/Buildings/BuildingMaster_BP.ConstructionProxy` _returnvalue))
      (`self.OpenTickGate`))
    (:`then_1`
      (`self.K2_DestroyActor` _returnvalue))))

(event `self.ReceiveTick`
  (params (DeltaSeconds :type "Float (single-precision)"))
  (`/Engine/EditorBlueprintResources/StandardMacros.Gate` true :!label _label
    (:`Exit`
      (`self.K2_SetActorLocation` self (`self.SetGridSnap`) false false))))

(event `OpenTickGate`
  (goto _label :!via `Open`))

(event `CloseTickGate`
  (goto _label :!via `Close`))

(fn `SetGridSnap`
  (returns (GridSnap :type "Vector Structure"))
  (bind (_cursorworldposition_x _cursorworldposition_y _cursorworldposition_z) (`KismetMathLibrary.BreakVector` (`self.CursorWorldPosition`)))
  (bind _gridsize (`self.GridSize`))
  (return (`KismetMathLibrary.MakeVector` (`/Game/RTS/Libraries/RTS_FunctionLibrary.GridSnap` _cursorworldposition_x _gridsize) (`/Game/RTS/Libraries/RTS_FunctionLibrary.GridSnap` _cursorworldposition_y _gridsize) (`/Game/RTS/Libraries/RTS_FunctionLibrary.GridSnap` _cursorworldposition_z _gridsize))))

(fn `UserConstructionScript`)