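; RTS player controller that sets up the god's-eye camera, building and HUD systems at game start.
; BeginPlay caches the GodsEye pawn, spawns construction manager and ghost building actors, sets locked-mouse Game and UI input, then creates the HUD.
; Helper functions derive move speed from spring arm length and screen-edge scroll speeds from mouse position.
; The MovementX/Y and PanX/Y graphs hold only unconnected transform and rotation math.
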(event `self.ReceiveBeginPlay`
  (bind _returnvalue (`KismetMathLibrary.MakeTransform` (0.0 0.0 0.0)))
  ;[1 1 1] Begin play
  (`|ExecutionSequence`
    (:`then_0`
      (`self.ReferenceCasts`))
    (:`then_1`
      (bind _returnvalue_2 (`|SpawnActorFromClass` "/Game/RTS/Blueprints/Construction/ConstructionManager_BP.ConstructionManager_BP_C" _returnvalue "AlwaysSpawn" "OverrideRootScale" null null))
      (set `self.ConstructionManagerRef` _returnvalue_2))
    (:`then_2`
      (bind _returnvalue_3 (`|SpawnActorFromClass` "/Game/RTS/Blueprints/Buildings/GhostBuilding_BP.GhostBuilding_BP_C" _returnvalue "AlwaysSpawn" "OverrideRootScale" null self (`self.CameraPawnRef`) null))
      (set `self.GhostBuildingRef` _returnvalue_3))
    (:`then_3`
      (`WidgetBlueprintLibrary.SetInputMode_GameAndUIEx` self (`self.GodsEyeHUD Reference`) "LockAlways" false)
      (`self.Create HUD`))))

(fn `MovementSpeedCalc`
  (returns (MoveSensitivity :type "Float (double-precision)"))
  (return (`KismetMathLibrary.FClamp` (/ (`SpringArmComponent.TargetArmLength` (`/Game/RTS/Blueprints/GodsEye_Pawn.SpringArm` (`self.CameraPawnRef`))) 100.0) 5.0 20.0)))

(fn `UserConstructionScript`)