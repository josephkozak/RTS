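; God's-eye RTS camera pawn that handles map navigation and positions the building placement ghost.
; Axis input and screen-edge scrolling move the pawn, with a Shift boost and keyboard speed scaled by spring-arm zoom.
; Holding Pan opens gates for mouse yaw and clamped pitch while blocking movement; Camera Reset restores pitch and zoom.
; In build mode, Tick feeds the cursor's world position to the controller's ghost, which Deselect kills.
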(event `InputAxis|MoveForward`
  (params (AxisValue :type "Float (single-precision)"))
  ;[1 1 1] Camera Movement
  ;;[1 1 1] Movement X
  (if (not (`self.DisableCamNav`))
    (`self.K2_SetActorTransform` (`self.Movement X` (`self.MovementSpeedCalc`) (`self.FastMoveMultiplier`) AxisValue) true)))

(event `Key|LeftShift`
  (params (Key :type "Key Structure"))
  ;[1 1 1] Camera Movement
  ;;[1 1 1] Speed Multiplier
  (:`Pressed`
    (set `self.FastMoveMultiplier` 5.0))
  (:`Released`
    (set `self.FastMoveMultiplier` 1.0)))

(event `InputAxis|MoveRight`
  (params (AxisValue :type "Float (single-precision)"))
  ;[1 1 1] Camera Movement
  ;;[1 1 1] Movement Y
  (if (not (`self.DisableCamNav`))
    (`self.K2_SetActorTransform` (`self.Movement Y` (`self.MovementSpeedCalc`) (`self.FastMoveMultiplier`) AxisValue) true)))

(event `InputAxisKey|MouseX`
  (params (AxisValue :type "Float (single-precision)"))
  ;[1 1 1] Camera Movement
  ;;[1 1 1] Edge Movement
  (if (not (`self.DisableCamNav`))
    (bind (_delta_x_speed _delta_y_speed) (`self.ScreenEdgeMovement` :!label _label))
    (`self.K2_AddActorLocalOffset` (`KismetMathLibrary.MakeVector` _delta_x_speed _delta_y_speed) true)))

(event `InputAxisKey|MouseX`
  (params (AxisValue :type "Float (single-precision)"))
  ;[1 1 1] Camera Movement
  ;;[1 1 1] Panning X
  (`/Engine/EditorBlueprintResources/StandardMacros.Gate` true :!label _label_2
    (:`Exit`
      (`self.K2_SetActorRotation` (`self.PanX` AxisValue (`self.PanSensitivity`))))))

(event `InputAxisKey|MouseY`
  (params (AxisValue :type "Float (single-precision)"))
  ;[1 1 1] Camera Movement
  ;;[1 1 1] Edge Movement
  (if (not (`self.DisableCamNav`))
    (goto _label :!via `MouseY`)))

(event `InputAction|Pan`
  (params (Key :type "Key Structure"))
  ;[1 1 1] Camera Movement
  ;;[1 1 1] Panning X
  (:`Pressed`
    (set `self.DisableCamNav` true)
    (goto _label_2 :!via `Open`))
  (:`Released`
    (set `self.DisableCamNav` false)
    (goto _label_2 :!via `Close`)))

(event `InputAxisKey|MouseY`
  (params (AxisValue :type "Float (single-precision)"))
  ;[1 1 1] Camera Movement
  ;;[1 1 1] Panning Y
  (`/Engine/EditorBlueprintResources/StandardMacros.Gate` true :!label _label_3
    (:`Exit`
      (`self.K2_SetActorRotation` (`self.PanY` AxisValue (`self.PanSensitivity`))))))

(event `InputAction|Pan`
  (params (Key :type "Key Structure"))
  ;[1 1 1] Camera Movement
  ;;[1 1 1] Panning Y
  (:`Pressed`
    (set `self.DisableCamNav` true)
    (goto _label_3 :!via `Open`))
  (:`Released`
    (set `self.DisableCamNav` false)
    (goto _label_3 :!via `Close`)))

(event `InputAction|Camera Reset`
  (params (Key :type "Key Structure"))
  ;[1 1 1] Camera Movement
  ;;[1 1 1] Reset Rotation
  (:`Pressed`
    (`self.K2_SetActorRotation` (`KismetMathLibrary.MakeRotator` (.roll (`self.K2_GetActorRotation`)) 0.0 (.yaw (`self.K2_GetActorRotation`))))
    (set `SpringArmComponent.TargetArmLength` 1500.0 (`self.SpringArm`))))

(event `InputAction|Zoom In`
  (params (Key :type "Key Structure"))
  ;[1 1 1] Camera Movement
  ;;[1 1 1] Zoom In
  (:`Pressed`
    (set `SpringArmComponent.TargetArmLength` (`KismetMathLibrary.FClamp` (- (`SpringArmComponent.TargetArmLength` (`self.SpringArm`)) (`self.ZoomSensitivity`)) 500.0 (`self.MaxArmDistance`)) (`self.SpringArm`))))

(event `InputAction|Zoom Out`
  (params (Key :type "Key Structure"))
  ;[1 1 1] Camera Movement
  ;;[1 1 1] Zoom Out
  (:`Pressed`
    (set `SpringArmComponent.TargetArmLength` (`KismetMathLibrary.FClamp` (+ (`SpringArmComponent.TargetArmLength` (`self.SpringArm`)) (`self.ZoomSensitivity`)) 500.0 (`self.MaxArmDistance`)) (`self.SpringArm`))))

(event `self.ReceiveBeginPlay`
  (bind _asrtsplayer_controller (cast `/Game/RTS/Blueprints/RTSPlayer_Controller` (`GameplayStatics.GetPlayerController` 0)))
  (set `self.ControllerReference` _asrtsplayer_controller)
  (set `self.GhostBuildingReference` (`/Game/RTS/Blueprints/RTSPlayer_Controller.GhostBuildingRef` _asrtsplayer_controller)))

(event `InputAction|Deselect`
  (params (Key :type "Key Structure"))
  (:`Pressed`
    (if (`self.BuildModeActive`)
      (`/Game/RTS/Blueprints/Buildings/GhostBuilding_BP.KillGhost` (`self.GhostBuildingReference`))
      (set `self.BuildModeActive` false))))

(event `self.ReceiveTick`
  (params (DeltaSeconds :type "Float (single-precision)"))
  ;[1 1 1] Building Ghost
  (if (`self.BuildModeActive`)
    (if (!= (`self.GhostBuildingReference`) null)
      (bind _output_get (set `/Game/RTS/Blueprints/Buildings/GhostBuilding_BP.CursorWorldPosition` (`/Game/RTS/Libraries/RTS_FunctionLibrary.GetCursorWorldPosition` (`self.ControllerReference`) (`self.SetSightDistance`)) (`self.GhostBuildingReference`)))
      (else
        (`KismetSystemLibrary.PrintString` "Failed reference to building")))))

(fn `MovementSpeedCalc`
  (returns (MoveSensitivity :type "Float (double-precision)"))
  (return (`KismetMathLibrary.FClamp` (/ (`SpringArmComponent.TargetArmLength` (`self.SpringArm`)) 100.0) 5.0 20.0)))

(fn `SetSightDistance`
  (returns (`Sight Distance` :type "Float (double-precision)"))
  (return (+ (`self.SightDistance`) (`SpringArmComponent.TargetArmLength` (`self.SpringArm`)))))

(fn `UserConstructionScript`)